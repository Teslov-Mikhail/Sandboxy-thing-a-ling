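; BP_Survivor is a pawn Blueprint with an inventory component, and its only active logic reports inventory changes as debug chat messages.
; When BP_Inventory fires InventoryChanged, it casts its controller to BP_SurvivalPlayerController and sends the action, item class name and stack amount to PrintDebugToChat.
; BeginPlay, overlap and Tick are disabled placeholders, and the construction script only calls its parent.
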(event InventoryChanged(BP_Inventory)
  (params (Action :type Enum_InventoryAction%20Enum :default "NewEnumerator0") (Stack :type Struct%20Item%20Stack%20Structure))
  (bind (_item _amount) (Utilities|Struct|BreakStruct_ItemStack Stack))
  (bind _asbp_survival_player_controller (Utilities|Casting|CastToBP_SurvivalPlayerController (Pawn|GetController)))
  (Default|PrintDebugtoChat _asbp_survival_player_controller (Utilities|String|Append (Utilities|String|EnumtoString Action) " " (Utilities|GetClassDisplayName _item) "" (Utilities|String|ToString(Integer) _amount))))

(event EventBeginPlay
  (|CallParentFunction) ; This node is disabled and will not be called.\nDrag off pins to build functionality.
)

(event Collision|EventActorBeginOverlap
  (params (OtherActor :type Actor%20Object%20Reference))
  (|CallParentFunction OtherActor) ; This node is disabled and will not be called.\nDrag off pins to build functionality.
)

(event EventTick
  (params (DeltaSeconds :type Float%20%28single-precision%29))
  (|CallParentFunction DeltaSeconds) ; This node is disabled and will not be called.\nDrag off pins to build functionality.
)

(fn ConstructionScript
  (|CallParentFunction))