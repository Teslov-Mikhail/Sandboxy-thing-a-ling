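; BP_BuildingTemplate is a building placement preview that shows a mesh tinted by whether its placement is correct.
; On BeginPlay it creates a dynamic instance of M_Template.
; Setup assigns the given static mesh and applies that material to every slot.
; SetState switches the material's Color parameter between blue for correct and red for incorrect.
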(event Custom|Set%20up
  (params (Mesh :type Static%20Mesh%20Object%20Reference))
  (Components|StaticMesh|SetStaticMesh (Variables|Default|GetMesh) Mesh)
  (for (_ _array_index) (Rendering|Material|GetMaterials (Variables|Default|GetMesh))
    (Rendering|Material|SetMaterial (Variables|Default|GetMesh) _array_index (Variables|Default|GetMaterial))))

(event Custom|Set%20State
  (params (Correct :type Boolean))
  (Rendering|Material|SetVectorParameterValue (Variables|Default|GetMaterial) "Color" (select Correct "(R=0.050980,G=0.137255,B=0.494118,A=1.000000)" "(R=0.356863,G=0.062745,B=0.043137,A=1.000000)") :!class /Script/Engine.MaterialInstanceDynamic))

(event EventBeginPlay
  (bind _returnvalue (Rendering|Material|CreateDynamicMaterialInstance "/Game/Mordhau/Maps/TesTest/assets/Blueprints/BuildingParts/M_Template.M_Template" "None" :!class /Script/Engine.KismetMaterialLibrary))
  (Variables|Default|SetMaterial _returnvalue))

(fn ConstructionScript)