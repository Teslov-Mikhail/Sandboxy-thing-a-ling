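; BP_BuildingPart is a building piece actor that supplies typed snap points, apparently for aligning other pieces to it.
; FindClosestSnapPoint picks the Box Component nearest a given location.
; FindSnapPoint then searches that box's direct children for a BP_SnapPoint of the requested type, returning its world location, rotation and component.
; The event graph and construction script add no behavior.
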(event EventBeginPlay
  (|CallParentFunction) ; This node is disabled and will not be called.\nDrag off pins to build functionality.
)

(event Collision|EventActorBeginOverlap
  (params (OtherActor :type Actor%20Object%20Reference))
  (|CallParentFunction OtherActor) ; This node is disabled and will not be called.\nDrag off pins to build functionality.
)

(event EventTick
  (params (DeltaSeconds :type Float%20%28single-precision%29))
  (|CallParentFunction DeltaSeconds))

(fn ConstructionScript
  (|CallParentFunction))

(fn FindClosestSnapPoint
  (params (Location :type Vector))
  (for _array_element (Actor|GetComponentsByClass "/Script/Engine.BoxComponent")
    (Math|Float|CompareFloat (Math|Vector|VectorLength (- Location (Transformation|GetWorldLocation _array_element))) (LocalVariables|GetClosest%20Distance)
      (:<
        (LocalVariables|SetClosest%20Distance (Math|Vector|VectorLength (- Location (Transformation|GetWorldLocation _array_element))))
        (LocalVariables|SetClosest%20Snap%20Point _array_element))))
  (Utilities|IsValid (LocalVariables|GetClosest%20Snap%20Point)
    (:Is%20Valid
      (return (LocalVariables|GetClosest%20Snap%20Point) true))
    (:Is%20Not%20Valid
      (return 0 false))))

(fn FindSnapPoint
  (params (Current%20Location :type Vector) (Type :type Enum_BuildTypes%20Enum :default "NewEnumerator0"))
  (bind (_snap_point _found) (CallFunction|FindClosestSnapPoint Current%20Location))
  (if _found
    (for _array_element (Components|GetChildrenComponents _snap_point false)
      (bind _asbp_snap_point (Utilities|Casting|CastToBP_SnapPoint _array_element))
      (if (Utilities|Enum|Equal(Enum) (Variables|/Game/Mordhau/Maps/TesTest/assets/Blueprints/BuildingParts/BP_SnapPoint.BP_SnapPoint_C|GetType _asbp_snap_point) Type)
        (return (Transformation|GetWorldLocation _array_element) (Transformation|GetWorldRotation _array_element) _asbp_snap_point)))
    (return "0, 0, 0" "0, 0, 0" 0)))