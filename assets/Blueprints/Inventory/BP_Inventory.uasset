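; Inventory component that stores item stacks (item class plus amount) in a Content array on its owning actor.
; Adding merges into an existing stack of the same class, while removing subtracts the amount and clears empty slots.
; Both broadcast InventoryChanged, though removal reads the slot after clearing, so its payload can be wrong.
; Dropping by index or class spawns the item actor in front of the owner, then removes that stack.
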(event Custom|Event%20Drop%20Item
  (params (Index :type Integer))
  (CallFunction|DropItembyIndex (Actor|GetComponentbyClass (Components|GetOwner) "BP_Inventory_C") Index))

(event EventBeginPlay)

(event EventTick
  (params (DeltaSeconds :type Float%20%28single-precision%29)))

(fn AddItem
  (params (Stack :type Struct%20Item%20Stack%20Structure))
  (bind (_item _amount) (Utilities|Struct|BreakStruct_ItemStack Stack))
  (bind _content (Variables|Default|Getcontent))
  (bind _array_index (CallFunction|FindItemIndexbyClass _item))
  (if (== _array_index -1)
    (bind _returnvalue (Utilities|Array|Add _content Stack))
    (Default|CallInventoryChanged "NewEnumerator0" Stack)
    (return _returnvalue)
    (else
      (|SetBy-RefVar (.Amount (Utilities|Struct|BreakStruct_ItemStack (Utilities|Array|Get(acopy) _content _array_index))) (+ (.Amount (Utilities|Struct|BreakStruct_ItemStack (Utilities|Array|Get(acopy) _content _array_index))) _amount))
      (Default|CallInventoryChanged "NewEnumerator0" (Utilities|Array|Get(acopy) _content _array_index))
      (return _array_index))))

(fn FindItemIndexbyClass
  (params (Class :type BP%20Item%20Class%20Reference))
  (for (_array_element _array_index) (Variables|Default|Getcontent)
    (if (== (.Item (Utilities|Struct|BreakStruct_ItemStack _array_element)) Class)
      (return _array_index)))
  (return -1))

(fn DropItembyClass
  (params (Class :type BP%20Item%20Class%20Reference))
  (bind _array_index (CallFunction|FindItemIndexbyClass Class))
  (CallFunction|DropItembyIndex _array_index))

(fn DropItembyIndex
  (params (Index :type Integer))
  (CallFunction|DropItem (Utilities|Array|Get(acopy) (Variables|Default|Getcontent) Index)))

(fn RemoveItems
  (params (Stack :type Struct%20Item%20Stack%20Structure))
  (bind (_item _amount) (Utilities|Struct|BreakStruct_ItemStack Stack))
  (bind _array_index (CallFunction|FindItemIndexbyClass _item))
  (if (!= _array_index -1)
    (|SetBy-RefVar (.Amount (Utilities|Struct|BreakStruct_ItemStack (Utilities|Array|Get(acopy) (Variables|Default|Getcontent) _array_index))) (- (.Amount (Utilities|Struct|BreakStruct_ItemStack (Utilities|Array|Get(acopy) (Variables|Default|Getcontent) _array_index))) _amount))
    (CallFunction|ClearEmptySlots)
    (Default|CallInventoryChanged "NewEnumerator1" (Utilities|Array|Get(acopy) (Variables|Default|Getcontent) _array_index))))

(fn ClearEmptySlots
  (for (_array_element _array_index) (Variables|Default|Getcontent)
    (if (== (.Amount (Utilities|Struct|BreakStruct_ItemStack _array_element)) 0)
      (Utilities|Array|RemoveIndex (Variables|Default|Getcontent) _array_index))))

(fn DropItem
  (params (Stack :type Struct%20Item%20Stack%20Structure%20%28by%20ref%29))
  (bind (_item _amount) (Utilities|Struct|BreakStruct_ItemStack Stack))
  (bind _returnvalue (Components|GetOwner))
  (Game|SpawnActorfromClass _item (Math|Transform|MakeTransform (+ (Transformation|GetActorLocation _returnvalue) (* (Transformation|GetActorForwardVector _returnvalue) 100))) "Undefined" _returnvalue _amount 0)
  (CallFunction|RemoveItems Stack))