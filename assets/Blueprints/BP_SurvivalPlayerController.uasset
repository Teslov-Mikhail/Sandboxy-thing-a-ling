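; Player controller for a survival mode on Mordhau that adds a toggleable inventory HUD.
; After possession it binds to the pawn's BP_Inventory change event, regenerating the widget's item list and posting a debug message to the Mordhau chatbox.
; The I key lazily creates the widget, then shows or hides it, switching cursor, input mode and move/look blocking through ToggleCursor.
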(event Custom|Reload%20Inventory
  (params (Action :type Enum_InventoryAction%20Enum :default "NewEnumerator0") (Stack :type Struct%20Item%20Stack%20Structure))
  (Default|GenerateItemList (Variables|/Game/Mordhau/Maps/TesTest/assets/Blueprints/Inventory/InventoryWidget/W_InventoryHUD.W_InventoryHUD_C|GetW_Inventory (Variables|Default|GetW_Inventory)))
  (CallFunction|PrintDebugtoChat "Kurwa jego mać"))

(event Custom|Print%20debug%20to%20chat
  (params (InString :type String))
  (bind _asbp_mordhau_hud (Utilities|Casting|CastToBP_MordhauHUD (HUD|GetHUD)))
  (Default|SendMessagetoChatbox _asbp_mordhau_hud "DEBUG" (Utilities|Text|ToText(String) InString)))

(event EventBeginPlay
  (|CallParentFunction))

(event EventOnAfterPossess
  (params (APawn :type Pawn%20Object%20Reference))
  (|CallParentFunction APawn)
  (EventDispatchers|BindEventtoInventoryChanged (Actor|GetComponentbyClass APawn "/Game/Mordhau/Maps/TesTest/assets/Blueprints/Inventory/BP_Inventory.BP_Inventory_C") (delegate Custom|Reload%20Inventory)))

(event Input|KeyboardEvents|I
  (params (Key :type Key%20Structure))
  (:Released
    (bind _w_inventory (Variables|Default|GetW_Inventory)
      (:then
        (if (Widget|IsVisible _w_inventory)
          (Widget|RemovefromParent (stale _output_get))
          (CallFunction|ToggleCursor)
          (else
            (UserInterface|Viewport|AddtoViewport (stale _output_get) 10000 :!label _label)
            (CallFunction|ToggleCursor (stale _output_get)))))
      (:else
        (bind _returnvalue (UserInterface|CreateWidget "/Game/Mordhau/Maps/TesTest/assets/Blueprints/Inventory/InventoryWidget/W_InventoryHUD.W_InventoryHUD_C" self))
        (bind _output_get (Variables|Default|SetW_Inventory _returnvalue))
        (goto _label)))))

(fn ConstructionScript
  (|CallParentFunction))

(fn ToggleCursor
  (params (Widget :type Widget%20Object%20Reference))
  (bind _returnvalue (Utilities|IsValid Widget))
  (bind _self self)
  (Variables|Default|SetbShowMouseCursor _returnvalue)
  (Input|SetIgnoreMoveInput _returnvalue)
  (Input|SetIgnoreLookInput _returnvalue)
  (if _returnvalue
    (Input|SetInputModeGameandUI _self Widget "DoNotLock" false)
    (else
      (Input|SetInputModeGameOnly _self))))